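; BP_PlayerBullet is a player-fired laser projectile that damages enemies on contact.
; The BulletOnSpawn event sets the ProjectileMovement velocity from a given direction and BulletSpeed.
; When LaserBullet overlaps an actor tagged Enemy, it prints a debug string, applies fixed damage, spawns an explosion emitter and destroys itself.
; Overlaps with untagged actors are ignored.
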(event OnComponentBeginOverlap(LaserBullet)
  (params (OverlappedComponent :type Primitive%20Component%20Object%20Reference) (OtherActor :type Actor%20Object%20Reference) (OtherComp :type Primitive%20Component%20Object%20Reference) (OtherBodyIndex :type Integer) (bFromSweep :type Boolean) (SweepResult :type Hit%20Result%20Structure%20%28by%20ref%29))
  (if (Actor|ActorHasTag OtherActor "Enemy")
    (Development|PrintString "Hello")
    (Game|Damage|ApplyDamage OtherActor 1.0 0 0)
    (Effects|SpawnEmitteratLocation "/Game/Particles/P_Explosion.P_Explosion" (Transformation|GetActorLocation))
    (Actor|DestroyActor)))

(event Custom|Bullet%20On%20Spawn
  (params (Direction :type Vector))
  (Variables|/Script/Engine.MovementComponent|SetVelocity (Variables|Default|GetProjectileMovement) (* Direction (Variables|Default|GetBullet%20Speed))))

(fn ConstructionScript)