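; BP_EnemyParent is a base enemy Blueprint that deals collision damage and destroys itself on contact.
; When EnemyBody overlaps a component tagged "Body", it applies CollisionDamage to the other actor and calls Death.
; The UpdateOwner event also calls Death when it reports the target is dead.
; Death spawns a scaled-up explosion emitter at the enemy's location and destroys the actor.
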(event OnComponentBeginOverlap(EnemyBody)
  (params (OverlappedComponent :type Primitive%20Component%20Object%20Reference) (OtherActor :type Actor%20Object%20Reference) (OtherComp :type Primitive%20Component%20Object%20Reference) (OtherBodyIndex :type Integer) (bFromSweep :type Boolean) (SweepResult :type Hit%20Result%20Structure%20%28by%20ref%29))
  (if (Components|ComponentHasTag OtherComp "Body")
    (Game|Damage|ApplyDamage OtherActor (Variables|Default|GetCollision%20Damage) 0 0)
    (CallFunction|Death)))

(event EventUpdateOwner
  (params (Health :type Float%20%28double-precision%29) (Is%20Target%20Dead? :type Boolean))
  (if Is%20Target%20Dead?
    (CallFunction|Death)))

(fn ConstructionScript)

(fn Death
  (Effects|SpawnEmitteratLocation "/Game/StarterContent/Particles/P_Explosion.P_Explosion" (Transformation|GetActorLocation) "0, 0, 0" "6.000000,6.000000,6.000000")
  (Actor|DestroyActor))