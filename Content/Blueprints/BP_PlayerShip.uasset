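; Player-controlled ship pawn that flies with mouse look and keyboard movement along its forward, right and up axes.
; BeginPlay possesses the pawn and adds the gameplay widget; key flags feed MovementMath, which drives FloatingPawnMovement each Tick.
; Tick also eases the body into a tilt when strafing and shows trails while moving.
; Sprint raises max speed and plays a reversible timeline that scales thrusters and widens camera FOV, but release never restores the speed.
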(event Custom|Stop%20Sprint%20Effect
  (bind _sprint_alpha (Timeline|TL_Sprint Reverse)
    (:Update
      (Transformation|SetWorldScale3D (Variables|Default|GetP_Thruster%20R) (Math|Vector|Lerp(Vector) "0.250000,0.500000,0.500000" "0.500000,0.500000,1.500000" _sprint_alpha))
      (Camera|SetFieldOfView (Variables|Default|GetCamera) (Math|Float|Lerp 9e+01 1.2e+02 _sprint_alpha)))))

(event Custom|Start%20Sprint%20Effect
  (bind _sprint_alpha (Timeline|TL_Sprint Play)
    (:Update
      (Transformation|SetWorldScale3D (Variables|Default|GetP_Thruster%20R) (Math|Vector|Lerp(Vector) "0.250000,0.500000,0.500000" "0.500000,0.500000,1.500000" _sprint_alpha))
      (Camera|SetFieldOfView (Variables|Default|GetCamera) (Math|Float|Lerp 9e+01 1.2e+02 _sprint_alpha)))))

(event EventBeginPlay
  (Pawn|Possess (Game|GetPlayerController 0) self)
  (Variables|Default|SetOriginal%20Body%20%20Relative%20Rotation (Variables|/Script/Engine.SceneComponent|GetRelativeRotation (Variables|Default|GetBody)))
  (bind _returnvalue (UserInterface|CreateWidget "/Game/UI/WG_Gameplay.WG_Gameplay_C" (Game|GetPlayerController 0)))
  (bind _output_get (Variables|Default|SetWG%20GamePlay _returnvalue))
  (UserInterface|Viewport|AddtoViewport _output_get 0))

(event Collision|EventActorBeginOverlap
  (params (OtherActor :type Actor%20Object%20Reference)))

(event EventTick
  (params (DeltaSeconds :type Float%20%28single-precision%29))
  (Utilities|FlowControl|Sequence
    (:then_0
      (Class|PawnMovementComponent|AddInputVector (Variables|Default|GetFloatingPawnMovement) (CallFunction|MovementMath) false))
    (:then_1
      (CallFunction|RotateShopwhenStrafe)
      (Rendering|SetVisibility (Variables|Default|GetNS_Trail%20L) (not (Utilities|Operators|EqualEqual :A (Transformation|GetVelocity))) false))))

(event Input|MouseEvents|MouseX
  (params (AxisValue :type Float%20%28single-precision%29))
  (Pawn|Input|AddControllerYawInput (* AxisValue 0.5)))

(event Input|MouseEvents|MouseY
  (params (AxisValue :type Float%20%28single-precision%29))
  (Pawn|Input|AddControllerPitchInput (* (* AxisValue -1.0) 0.5)))

(event Input|KeyboardEvents|W
  (params (Key :type Key%20Structure :default "None"))
  ;[1 1 1] Set input
  (:Pressed
    (Variables|Default|SetW%20is%20Pressed true))
  (:Released
    (Variables|Default|SetW%20is%20Pressed false)))

(event Input|KeyboardEvents|D
  (params (Key :type Key%20Structure :default "None"))
  ;[1 1 1] Set input
  (:Pressed
    (Variables|Default|SetD%20is%20Pressed true))
  (:Released
    (Variables|Default|SetD%20is%20Pressed false)))

(event Input|KeyboardEvents|S
  (params (Key :type Key%20Structure :default "None"))
  ;[1 1 1] Set input
  (:Pressed
    (Variables|Default|SetS%20is%20Pressed true))
  (:Released
    (Variables|Default|SetS%20is%20Pressed false)))

(event Input|KeyboardEvents|SpaceBar
  (params (Key :type Key%20Structure :default "None"))
  ;[1 1 1] Set input
  (:Pressed
    (Variables|Default|SetSpace%20is%20Pressed true))
  (:Released
    (Variables|Default|SetSpace%20is%20Pressed false)))

(event Input|KeyboardEvents|LeftCtrl
  (params (Key :type Key%20Structure :default "None"))
  ;[1 1 1] Set input
  (:Pressed
    (Variables|Default|SetLeft%20Control%20is%20Pressed true))
  (:Released
    (Variables|Default|SetLeft%20Control%20is%20Pressed false)))

(event Input|KeyboardEvents|A
  (params (Key :type Key%20Structure :default "None"))
  ;[1 1 1] Set input
  (:Pressed
    (Variables|Default|SetA%20is%20pressed true))
  (:Released
    (Variables|Default|SetA%20is%20pressed false)))

(event Input|KeyboardEvents|LeftShift
  (params (Key :type Key%20Structure :default "None"))
  ;[1 1 1] Set input
  (:Pressed
    (Variables|Default|SetIs%20Sprinting true)
    (Variables|/Script/Engine.FloatingPawnMovement|SetMaxSpeed (Variables|Default|GetFloatingPawnMovement) 2.5e+03)
    (CallFunction|StartSprintEffect))
  (:Released
    (Variables|Default|SetIs%20Sprinting false)
    (CallFunction|StopSprintEffect)))

(fn ConstructionScript)

(fn MovementMath
  (bind _returnvalue (Transformation|GetActorForwardVector))
  (bind _returnvalue_2 (Transformation|GetActorRightVector))
  (bind _returnvalue_3 (Transformation|GetActorUpVector))
  (Variables|Default|SetDirection%20FB (select (or (and (Variables|Default|GetW%20is%20Pressed) (Variables|Default|GetS%20is%20Pressed)) (and (not (Variables|Default|GetW%20is%20Pressed)) (not (Variables|Default|GetS%20is%20Pressed)))) "0, 0, 0" (Math|Vector|SelectVector (* _returnvalue -1) _returnvalue (Variables|Default|GetS%20is%20Pressed))))
  (Variables|Default|SetDirection%20LR (select (or (and (Variables|Default|GetD%20is%20Pressed) (Variables|Default|GetA%20is%20pressed)) (and (not (Variables|Default|GetD%20is%20Pressed)) (not (Variables|Default|GetA%20is%20pressed)))) "0, 0, 0" (Math|Vector|SelectVector (* _returnvalue_2 -1) _returnvalue_2 (Variables|Default|GetA%20is%20pressed))))
  (Variables|Default|SetDirection%20UD (select (or (and (Variables|Default|GetSpace%20is%20Pressed) (Variables|Default|GetLeft%20Control%20is%20Pressed)) (and (not (Variables|Default|GetSpace%20is%20Pressed)) (not (Variables|Default|GetLeft%20Control%20is%20Pressed)))) "0, 0, 0" (Math|Vector|SelectVector (* _returnvalue_3 -1) _returnvalue_3 (Variables|Default|GetLeft%20Control%20is%20Pressed))))
  (return (+ (Variables|Default|GetDirection%20FB) (Variables|Default|GetDirection%20LR) (Variables|Default|GetDirection%20UD))))

(fn RotateShopwhenStrafe
  (bind _body (Variables|Default|GetBody))
  (bind _original_body__relative_rotation (Variables|Default|GetOriginal%20Body%20%20Relative%20Rotation))
  (bind _body_2 (Variables|Default|GetBody))
  (if (or (and (Variables|Default|GetD%20is%20Pressed) (Variables|Default|GetA%20is%20pressed)) (and (not (Variables|Default|GetD%20is%20Pressed)) (not (Variables|Default|GetA%20is%20pressed))))
    (Transformation|SetRelativeRotation _body_2 (Math|Interpolation|RInterpTo (Variables|/Script/Engine.SceneComponent|GetRelativeRotation _body_2) (Variables|Default|GetOriginal%20Body%20%20Relative%20Rotation) (Utilities|Time|GetWorldDeltaSeconds) 1.0) false false)
    (else
      (Transformation|SetRelativeRotation _body (Math|Interpolation|RInterpTo (Variables|/Script/Engine.SceneComponent|GetRelativeRotation _body) (Math|Rotator|CombineRotators (Variables|Default|GetOriginal%20Body%20%20Relative%20Rotation) (Math|Rotator|SelectRotator (Math|Rotator|CombineRotators _original_body__relative_rotation "0.000000,0.000000,-15.000000") (Math|Rotator|CombineRotators _original_body__relative_rotation "0.000000,0.000000,15.000000") (Variables|Default|GetA%20is%20pressed))) (Utilities|Time|GetWorldDeltaSeconds) 1.0) false false))))