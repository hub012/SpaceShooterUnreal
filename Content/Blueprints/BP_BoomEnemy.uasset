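; BP_BoomEnemy is an enemy actor that constantly homes in on the player pawn.
; Each Tick it moves toward the first player's location at a constant Speed using VInterpToConstant and an unswept SetActorLocation, so movement ignores collision.
; On BeginPlay it binds RotatingMovement to EnemyBody, so only that component spins.
; The graph contains no explosion or damage logic, and its overlap event is an empty disabled stub.
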(event EventBeginPlay
  (Components|Movement|SetUpdatedComponent (Variables|Default|GetRotatingMovement) (Variables|Default|GetEnemy%20Body)))

(event Collision|EventActorBeginOverlap
  (params (OtherActor :type Actor%20Object%20Reference)))

(event EventTick
  (params (DeltaSeconds :type Float%20%28single-precision%29))
  (Transformation|SetActorLocation (Math|Interpolation|VInterptoConstant (Transformation|GetActorLocation) (Transformation|GetActorLocation (Game|Player|GetPlayerPawn 0)) DeltaSeconds (Math|Conversions|ToFloat(Integer) (Variables|Default|GetSpeed))) false false))

(fn ConstructionScript
  (|CallParentFunction))