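; BPC_Damageable is a component that gives its owning actor health that can be damaged and healed.
; On BeginPlay it binds to the owner's OnTakeAnyDamage, routing incoming damage into RemoveHealth.
; AddHealth and RemoveHealth clamp CurrentHealth between zero and MaxHealth, then report the new health and a dead flag to the owner through UpdateOwnerMessage.
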(event Custom|BindOfTakeAnyDamage
  (params (DamagedActor :type Actor%20Object%20Reference) (Damage :type Float%20%28single-precision%29) (DamageType :type Damage%20Type%20Object%20Reference) (InstigatedBy :type Controller%20Object%20Reference) (DamageCauser :type Actor%20Object%20Reference))
  (CallFunction|RemoveHealth Damage))

(event EventBeginPlay
  (EventDispatchers|BindEventtoOnTakeAnyDamage (Components|GetOwner) (delegate Custom|BindOfTakeAnyDamage)))

(fn AddHealth
  (params (Heal%20Amount :type Float%20%28double-precision%29))
  (Variables|Default|SetCurrent%20Health (Math|Float|Clamp(Float) (+ Heal%20Amount (Variables|Default|GetCurrent%20Health)) 0.0 (Variables|Default|GetMax%20Health)))
  (Class|BIComunications|UpdateOwner(Message) (Components|GetOwner) (Variables|Default|GetCurrent%20Health) (== (Variables|Default|GetCurrent%20Health) 0.0)))

(fn RemoveHealth
  (params (Damage :type Float%20%28double-precision%29))
  (Variables|Default|SetCurrent%20Health (Math|Float|Clamp(Float) (- (Variables|Default|GetCurrent%20Health) Damage) 0.0 (Variables|Default|GetMax%20Health)))
  (Class|BIComunications|UpdateOwner(Message) (Components|GetOwner) (Variables|Default|GetCurrent%20Health) (== (Variables|Default|GetCurrent%20Health) 0.0)))