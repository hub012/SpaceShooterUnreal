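; GM_SpaceGame is the game mode Blueprint for a space game that manages the main menu.
; On BeginPlay it creates the WG_MainMenu widget, stores a reference and shows it.
; Show and hide events add or remove the widget while toggling the mouse cursor and switching between UI-only and game-only input.
; A Spawnplayer event is declared but empty.
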(event Custom|Show%20main%20menu
  (bind _returnvalue (Game|GetPlayerController 0))
  (bind _wg_main_menu_ref (Variables|Default|GetWG%20Main%20Menu%20Ref))
  (Variables|/Script/Engine.PlayerController|SetbShowMouseCursor _returnvalue true)
  (Input|SetInputModeUIOnly _returnvalue _wg_main_menu_ref "DoNotLock" false)
  (UserInterface|Viewport|AddtoViewport _wg_main_menu_ref 0))

(event Custom|Hide%20main%20menu
  (bind _returnvalue (Game|GetPlayerController 0))
  (Variables|/Script/Engine.PlayerController|SetbShowMouseCursor _returnvalue false)
  (Input|SetInputModeGameOnly _returnvalue false)
  (Widget|RemovefromParent (Variables|Default|GetWG%20Main%20Menu%20Ref)))

(event Custom|Spawn%20player)

(event EventBeginPlay
  (bind _returnvalue (UserInterface|CreateWidget "/Game/UI/WG_MainMenu.WG_MainMenu_C" (Game|GetPlayerController 0)))
  (Variables|Default|SetWG%20Main%20Menu%20Ref _returnvalue)
  (CallFunction|ShowMainMenu))

(fn ConstructionScript)